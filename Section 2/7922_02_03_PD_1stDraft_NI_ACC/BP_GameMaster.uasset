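; BP_GameMaster tracks the player's score and the enemies remaining in the level.
; On BeginPlay it gathers all BP_Enemy actors and binds AddScore to each one's event dispatcher.
; AddScore increments the current score and removes the reported enemy from the list.
; It also passes itself as a reference to the UW_Scoreboard hosted by its Widget component.
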(event Custom|AddScore
  (params (EnemyToDelete :type BP%20Enemy%20Object%20Reference))
  (Math|Integer|IncrementInt (Variables|Default|GetCurrentScore)
    (:%20%20
      (Utilities|Array|RemoveItem (Variables|Default|GetEnemies) EnemyToDelete))))

(event EventBeginPlay
  (Utilities|FlowControl|Sequence
    (:then_0
      (bind _outactors (Actor|GetAllActorsOfClass "/Game/Core/BP_Enemy.BP_Enemy_C"))
      (bind _output_get (Variables|Default|SetEnemies _outactors))
      (for _array_element _output_get
        (EventDispatchers|BindEventtoAddScore _array_element (delegate Custom|AddScore))))
    (:then_1
      (bind _asuw_scoreboard (Utilities|Casting|CastToUW_Scoreboard (UserInterface|GetUserWidgetObject (Variables|Default|GetWidget))))
      (Variables|/Game/Widgets/UW_Scoreboard.UW_Scoreboard_C|SetGameMasterRef _asuw_scoreboard self))))

(event Collision|EventActorBeginOverlap
  (params (OtherActor :type Actor%20Object%20Reference)))

(event EventTick
  (params (DeltaSeconds :type Float%20%28single-precision%29)))

(fn ConstructionScript)