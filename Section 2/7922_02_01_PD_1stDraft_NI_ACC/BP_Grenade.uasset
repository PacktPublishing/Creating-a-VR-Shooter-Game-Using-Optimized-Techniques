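; Grenade actor that can be picked up, dropped, and explodes on a hard enough impact, killing nearby enemies.
; Pickup attaches the mesh to a given component with physics off, and Drop detaches it and restores physics.
; A hit impulse at or above a threshold spawns an explosion effect and hides the mesh.
; A zero-length multi-sphere trace then calls Die on BP_Enemy actors in range, and the grenade destroys itself after a short delay.
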(event OnComponentHit(SM_Grenade)
  (params (HitComponent :type Primitive%20Component%20Object%20Reference) (OtherActor :type Actor%20Object%20Reference) (OtherComp :type Primitive%20Component%20Object%20Reference) (NormalImpulse :type Vector) (Hit :type Hit%20Result%20Structure%20%28by%20ref%29))
  (bind _returnvalue (Transformation|GetActorLocation))
  (bind _sm_grenade (Variables|Default|GetSM_Grenade))
  (if (>= (Math|Vector|VectorLength NormalImpulse) (Variables|Default|GetForceNeededForExplosion))
    (Effects|SpawnEmitteratLocation "/Game/StarterContent/Particles/P_Explosion.P_Explosion" (Transformation|GetActorLocation))
    (Rendering|SetVisibility _sm_grenade false false)
    (Physics|SetSimulatePhysics _sm_grenade false)
    (Utilities|FlowControl|Sequence
      (:then_0
        (bind _outhits (Collision|MultiSphereTraceForObjects _returnvalue _returnvalue 1.5e+03 (Utilities|Array|MakeArray "ObjectTypeQuery2") false 0 "None"))
        (for _array_element _outhits
          (bind _asbp_enemy (Utilities|Casting|CastToBP_Enemy (.HitActor (Collision|BreakHitResult _array_element))))
          (Default|Die _asbp_enemy)))
      (:then_1
        (Utilities|FlowControl|Delay 0.5)
        (Actor|DestroyActor)))))

(event EventPickup
  (params (AttachTo :type Scene%20Component%20Object%20Reference))
  (bind _sm_grenade (Variables|Default|GetSM_Grenade))
  (Physics|SetSimulatePhysics _sm_grenade false)
  (Transformation|AttachComponentToComponent _sm_grenade AttachTo "None" "KeepWorld" "KeepWorld" "KeepWorld" false))

(event EventDrop
  (bind _sm_grenade (Variables|Default|GetSM_Grenade))
  (Physics|SetSimulatePhysics _sm_grenade true)
  (Transformation|DetachFromComponent _sm_grenade "KeepWorld" "KeepWorld" "KeepWorld" true))

(fn ConstructionScript)