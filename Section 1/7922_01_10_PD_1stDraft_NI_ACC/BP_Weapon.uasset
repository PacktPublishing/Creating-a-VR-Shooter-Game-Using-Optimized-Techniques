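; BP_Weapon is a hand-held weapon actor with pickup, drop and ammo reload handling.
; Pickup snaps the mesh to the holder's WeaponSocket, flipping it for a left-hand BP_MC, and Drop detaches it with physics restored.
; A bullet count widget holds a reference to the weapon and shows only while held.
; Overlapping a BP_AmmoBox with the reload box adds its ammo up to the maximum and destroys it.
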(event OnComponentBeginOverlap(ReloadCollisionBox)
  (params (OverlappedComponent :type Primitive%20Component%20Object%20Reference) (OtherActor :type Actor%20Object%20Reference) (OtherComp :type Primitive%20Component%20Object%20Reference) (OtherBodyIndex :type Integer) (bFromSweep :type Boolean) (SweepResult :type Hit%20Result%20Structure%20%28by%20ref%29))
  (bind _asbp_ammo_box (Utilities|Casting|CastToBP_AmmoBox OtherActor))
  (Variables|Default|SetBulletCount (Math|Integer|Clamp(Integer) (+ (Variables|/Game/Items/BP_AmmoBox.BP_AmmoBox_C|GetAmmoCount _asbp_ammo_box) (Variables|Default|GetBulletCount)) 0 (Variables|Default|GetMaxBulletCount)))
  (Actor|DestroyActor _asbp_ammo_box))

(event EventPickup
  (params (AttachTo :type Scene%20Component%20Object%20Reference))
  (bind _sm_weapon (Variables|Default|GetSM_Weapon))
  (Physics|SetSimulatePhysics _sm_weapon false)
  (Transformation|AttachComponentToComponent _sm_weapon AttachTo "WeaponSocket" "SnapToTarget" "SnapToTarget" "KeepRelative" false)
  (Rendering|SetVisibility (Variables|Default|GetBulletCountWidget) true false)
  (bind _asbp_mc (Utilities|Casting|CastToBP_MC (Components|GetOwner AttachTo)))
  (if (Utilities|Enum|Equal(Enum) (Variables|/Game/Core/BP_MC.BP_MC_C|GetHand _asbp_mc) "Left")
    (Transformation|SetRelativeRotation (Variables|Default|GetSM_Weapon) "180.000000, 0, 0" false false)))

(event EventBeginPlay
  (bind _asuw_weapon_bullet_count (Utilities|Casting|CastToUW_WeaponBulletCount (UserInterface|GetUserWidgetObject (Variables|Default|GetBulletCountWidget))))
  (Variables|/Game/Widgets/UW_WeaponBulletCount.UW_WeaponBulletCount_C|SetWeaponRef _asuw_weapon_bullet_count self)
  (Variables|Default|SetBulletCount (Variables|Default|GetMaxBulletCount)))

(event EventDrop
  (Physics|SetSimulatePhysics (Variables|Default|GetSM_Weapon) true)
  (Transformation|DetachFromActor "KeepWorld" "KeepWorld" "KeepWorld")
  (Rendering|SetVisibility (Variables|Default|GetBulletCountWidget) false false))

(fn ConstructionScript)